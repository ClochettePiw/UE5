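; BP_GravityCube is a cube actor whose gravity toggles each time the space bar is released.
; A GravityMultiplier float, reset to positive on BeginPlay, flips sign on each release to act as the toggle state.
; A positive value enables gravity on the cube and deactivates its PhysicsThruster; a negative one disables gravity and activates the thruster, with a debug print of the state.
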(event `self.ReceiveBeginPlay`
  (set `self.GravityMultiplier` 1.0))

(event `Key|SpaceBar`
  (params (Key :type "Key Structure"))
  (:`Released`
    (set `self.GravityMultiplier` (* (`self.GravityMultiplier`) -1.0))
    (if (> (`self.GravityMultiplier`) 0.0)
      (`PrimitiveComponent.SetEnableGravity` (`self.Cube`) true)
      (`ActorComponent.SetActive` (`self.PhysicsThruster`) false false)
      (`KismetSystemLibrary.PrintString` "Gravity true")
      (else
        (`PrimitiveComponent.SetEnableGravity` (`self.Cube`) false)
        (`ActorComponent.SetActive` (`self.PhysicsThruster`) true false)
        (`KismetSystemLibrary.PrintString` "Gravity false")))))

(fn `UserConstructionScript`)