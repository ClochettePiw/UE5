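; BP_Platform is a moving platform that travels along a configurable Direction at a set Speed.
; Tick offsets the actor without sweep, using Direction clamped per axis to ±1 but not normalized.
; Once it passes Distance from the BasePosition saved at BeginPlay, it either reverses and resets that base when CanLoop is set, or stops.
; The Calcul function is an uncalled stub returning false.
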(event `self.ReceiveBeginPlay`
  ;[0.004025 1 0 0.502] Set base position
  (set `self.BasePosition` (`self.K2_GetActorLocation`)))

(event `self.ReceiveTick`
  (params (DeltaSeconds :type "Float (single-precision)"))
  ;[0.004025 1 0 0.502] Movement
  (`self.K2_SetActorLocation` (+ (`self.K2_GetActorLocation`) (* (`self.ClampDirection`) (* DeltaSeconds (`self.Speed`)))))
  (if (> (`KismetMathLibrary.Vector_Distance` (`self.BasePosition`) (`self.K2_GetActorLocation`)) (`self.Distance`))
    (if (`self.CanLoop`)
      (set `self.Speed` (* (`self.Speed`) -1.0))
      (set `self.BasePosition` (`self.K2_GetActorLocation`))
      (else
        (set `self.Speed` 0.0)))))

(fn `Calcul`
  (params (NewParam :type Boolean))
  (returns (NewParam1 :type Boolean))
  (return false))

(fn `ClampDirection`
  (returns (Direction :type "Vector Structure"))
  (bind (_direction_x _direction_y _direction_z) (`KismetMathLibrary.BreakVector` (`self.Direction`)))
  (return (`KismetMathLibrary.MakeVector` (`KismetMathLibrary.FClamp` _direction_x -1.0) (`KismetMathLibrary.FClamp` _direction_y -1.0) (`KismetMathLibrary.FClamp` _direction_z -1.0))))

(fn `UserConstructionScript`)