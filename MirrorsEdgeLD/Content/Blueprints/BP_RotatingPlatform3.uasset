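; BP_RotatingPlatform3 is a rotating platform actor with a base and three platforms that begins moving on BeginPlay.
; It sets the base to its start rotation, then plays the TL_Rotation timeline.
; Each update, the timeline alpha lerps the base between its own start and target rotations.
; The same alpha lerps all three platforms between a separate shared start and target pair, in relative space.
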(event `self.ReceiveBeginPlay`
  (`SceneComponent.K2_SetRelativeRotation` (`self.Base`) (`self.StartRotation`) false false)
  (bind (_direction _alpha) (`Timeline|TL_Rotation`)
    (:`Update`
      (`SceneComponent.K2_SetRelativeRotation` (`self.Base`) (`KismetMathLibrary.RLerp` (`self.StartRotation`) (`self.TargetRotation`) _alpha) false false)
      (bind _returnvalue (`KismetMathLibrary.RLerp` (`self.PlatformStartRotation`) (`self.PlatformTargetRotation`) _alpha))
      (`SceneComponent.K2_SetRelativeRotation` (`self.Platform1`) _returnvalue false false)
      (`SceneComponent.K2_SetRelativeRotation` (`self.Platform2`) _returnvalue false false)
      (`SceneComponent.K2_SetRelativeRotation` (`self.Platform3`) _returnvalue false false))))

(fn `UserConstructionScript`)